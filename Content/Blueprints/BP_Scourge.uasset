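; BP_Scourge is an NPC with randomized combat stats and a sprite visual, built on a parent class.
; On BeginPlay it runs the parent logic, then rolls MaxHealth and Attack within fixed ranges and starts Health at full.
; Each Tick it checks the actor's yaw to determine facing and snaps the Sprite's world rotation to one of two fixed orientations.
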(event EventBeginPlay
  (|CallParentFunction)
  (bind _output_get (Variables|Default|SetMaxHealth (Math|Random|RandomIntegerinRange 30 50)))
  (Variables|Default|SetHealth _output_get)
  (Variables|Default|SetAttack (Math|Random|RandomIntegerinRange 30 40)))

(event EventTick
  (params (DeltaSeconds :type Float%20%28single-precision%29))
  (bind _returnvalue (Transformation|GetActorRotation))
  ;[0 1 0.7561] Determine which way is the npc is facing
  (if (or (>= (.yaw _returnvalue) 89.9) (<= (.yaw _returnvalue) -89.9))
    (Transformation|SetWorldRotation (Variables|Default|GetSprite) "0.000000,180.000000,0.000000" false false)
    (else
      (Transformation|SetWorldRotation (Variables|Default|GetSprite) "0.000000,90.000000,0.000000" false false))))

(fn ConstructionScript
  (|CallParentFunction))