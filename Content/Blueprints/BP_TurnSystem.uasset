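; Turn manager for grid combat that tracks whose turn it is and manages the main party.
; A unit-to-bool map serves as the turn queue, with NextTurn passing the active flag along and wrapping around.
; RequestMCTS flattens units, rotated to start from the active one, plus obstacles and traps into parallel primitive arrays as search input.
; CombatFinished clears combat state, notifies the player controller and grants the grid's rewards.
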(event Custom|AddUnit
  (params (Unit :type BP%20Entity%20Object%20Reference%20%28by%20ref%29))
  ;[1 1 1] Add unit to the turn system
  (if (Utilities|Map|IsEmpty (Variables|Default|GetUnits))
    (Utilities|Map|Add (Variables|Default|GetUnits) Unit true)
    (else
      (Utilities|Map|Add (Variables|Default|GetUnits) Unit false))))

(event Custom|CombatFinished
  (Utilities|Map|Clear (Variables|Default|GetUnits))
  (Utilities|Array|Clear (Variables|/Game/Blueprints/BP_Grid.BP_Grid_C|GetUnitsOnGrid (Variables|Default|GetGrid)))
  (for _array_element (Variables|Default|GetMainParty)
    (Variables|/Game/Blueprints/BP_Entity.BP_Entity_C|SetGrid _array_element 0))
  (bind _aspc_player_controller (Utilities|Casting|CastToPC_PlayerController (Game|GetPlayerController 0)))
  (Default|OnCombatFinished _aspc_player_controller)
  (Default|RewardPlayer _aspc_player_controller (Default|GetClearRewards (Variables|Default|GetGrid)))
  (Variables|Default|SetGrid 0))

(event Custom|StartTurnBase
  ;[1 1 1] Enable turn to be changed
  (bind _keys (Utilities|Map|Keys (Variables|Default|GetUnits)))
  (if (Utilities|Array|IsNotEmpty _keys)
    (Default|ChangeTurn (Utilities|Array|Get(acopy) _keys) true)
    (Variables|Default|SetTurnEnabled true)))

(event Custom|RemoveUnit
  (params (Key :type BP%20Entity%20Object%20Reference%20%28by%20ref%29))
  (Utilities|Map|Remove (Variables|Default|GetUnits) Key)
  (if (Variables|/Game/Blueprints/BP_Entity.BP_Entity_C|GetAlly? Key)
    (Utilities|Array|RemoveItem (Variables|Default|GetMainParty) Key)))

(event Custom|AddMainParty
  (params (Party%20Member :type BP%20Entity%20Object%20Reference%20%28by%20ref%29))
  (Utilities|Array|Add (Variables|Default|GetMainParty) Party%20Member))

(event Custom|MoveAllMainParty
  (params (NextSpot :type BP%20Gathering%20Point%20Object%20Reference))
  (for _array_element (Variables|Default|GetMainParty)
    (AI|Navigation|SimpleMovetoLocation (Pawn|GetController _array_element) (Default|GetValidPosition NextSpot))))

(event EventBeginPlay
  (bind _aspc_player_controller (Utilities|Casting|CastToPC_PlayerController (Game|GetPlayerController 0)))
  (Default|UpdateTurnManager _aspc_player_controller self))

(fn ConstructionScript)

(fn SetUp
  (params (Grid :type BP%20Grid%20Object%20Reference))
  (Variables|Default|SetGrid Grid))

(fn NextTurn
  (bind _units (Variables|Default|GetUnits))
  ;[1 1 1] Find who's turn is it
  (Default|CallNextTurnCalled)
  (bind _keys (Utilities|Map|Keys (Variables|Default|GetUnits)))
  (bind (_array_element _array_index) (Utilities|Array|ForEachLoopwithBreak _keys :!label _label)
    (:LoopBody
      (if (.Value (Utilities|Map|Find (Variables|Default|GetUnits) _array_element))
        ;[1 1 1] Change Turn
        (Default|ChangeTurn _array_element false)
        (Utilities|Map|Add (Variables|Default|GetUnits) _array_element false)
        (if (== _array_index (- (Utilities|Array|Length _keys) 1))
          (Utilities|Map|Add _units (Utilities|Array|Get(acopy) _keys) true)
          (Default|ChangeTurn (Utilities|Array|Get(acopy) _keys) true)
          (goto _label Break)
          (else
            (Utilities|Map|Add _units (Utilities|Array|Get(acopy) _keys (+ _array_index 1)) true)
            (Default|ChangeTurn (Utilities|Array|Get(acopy) _keys (+ _array_index 1)) true)
            (goto _label Break)))))))

(fn RequestMCTS
  (params (RequestingUnit :type BP%20Entity%20Object%20Reference))
  (Utilities|Array|Clear (LocalVariables|GetSortedUnits))
  (LocalVariables|SetNextUnitTurn 0)
  (LocalVariables|SetNextUnitIndex -1)
  (bind _keys (Utilities|Map|Keys (Variables|Default|GetUnits)))
  (bind _output_get (LocalVariables|SetUnsortedUnit _keys))
  (bind (_array_element _array_index) (Utilities|Array|ForEachLoopwithBreak _output_get)
    (:LoopBody
      ;[1 0.2661 0.6892] Find whose turn is it
      (if (.Value (Utilities|Map|Find (Variables|Default|GetUnits) _array_element))
        (bind _output_get_2 (LocalVariables|SetNextUnitTurn _array_element))
        (LocalVariables|SetNextUnitIndex _array_index)
        (Utilities|Array|Add (LocalVariables|GetSortedUnits) _output_get_2)
        (else
          ;[1 1 1] Add the next units in the turn queue
          (if (and (> _array_index (LocalVariables|GetNextUnitIndex)) (Utilities|IsValid (LocalVariables|GetNextUnitTurn)))
            (Utilities|Array|Add (LocalVariables|GetSortedUnits) _array_element)))))
    (:Completed
      ;[0.4242 0.4081 1] Add units from the one before the selected unit
      (for _index (range 0 (LocalVariables|GetNextUnitIndex))
        (if (< (Utilities|Array|FindItem (LocalVariables|GetSortedUnits) (Utilities|Array|Get(acopy) (LocalVariables|GetUnsortedUnit) _index)) 0)
          (Utilities|Array|Add (LocalVariables|GetSortedUnits) (Utilities|Array|Get(acopy) (LocalVariables|GetUnsortedUnit) _index))))
      ;[1 1 1] Setup primitives for input
      (Utilities|Array|Clear (LocalVariables|GetInputNPC))
      (Utilities|Array|Clear (LocalVariables|GetInputNPCTeams))
      (Utilities|Array|Clear (LocalVariables|GetInputPosX))
      (Utilities|Array|Clear (LocalVariables|GetInputPosY))
      (Utilities|Array|Clear (LocalVariables|GetInputMaxHealth))
      (Utilities|Array|Clear (LocalVariables|GetInputAttack))
      (Utilities|Array|Clear (LocalVariables|GetInputCurrentHealth))
      (for _array_element_2 (LocalVariables|GetSortedUnits)
        (Utilities|Array|Add (LocalVariables|GetInputNPC) (Variables|/Game/Blueprints/BP_Entity.BP_Entity_C|GetID _array_element_2))
        (if (Variables|/Game/Blueprints/BP_Entity.BP_Entity_C|GetAlly? _array_element_2)
          (Utilities|Array|Add (LocalVariables|GetInputNPCTeams) "Ally")
          (else
            (Utilities|Array|Add (LocalVariables|GetInputNPCTeams) "Enemy")))
        (Utilities|Array|Add (LocalVariables|GetInputPosX) (Math|Conversions|ToInteger(Byte) (Utilities|String|GetSubstring (Variables|/Game/Blueprints/BP_Entity.BP_Entity_C|GetPosition _array_element_2) 0 2)))
        (Utilities|Array|Add (LocalVariables|GetInputPosY) (Math|Conversions|ToInteger(Byte) (Utilities|String|GetSubstring (Variables|/Game/Blueprints/BP_Entity.BP_Entity_C|GetPosition _array_element_2) 2 2)))
        (Utilities|Array|Add (LocalVariables|GetInputMaxHealth) (Variables|/Game/Blueprints/BP_Entity.BP_Entity_C|GetMaxHealth _array_element_2))
        (Utilities|Array|Add (LocalVariables|GetInputCurrentHealth) (Variables|/Game/Blueprints/BP_Entity.BP_Entity_C|GetHealth _array_element_2))
        (Utilities|Array|Add (LocalVariables|GetInputAttack) (Variables|/Game/Blueprints/BP_Entity.BP_Entity_C|GetAttack _array_element_2)))
      ;[1 1 1] Put obstacles at last indexes
      (for _array_element_3 (Variables|/Game/Blueprints/BP_Grid.BP_Grid_C|GetGridsWithObstacles (Variables|Default|GetGrid))
        (Utilities|Array|Add (LocalVariables|GetInputNPC) "Obstacle")
        (Utilities|Array|Add (LocalVariables|GetInputNPCTeams) "Obstacle")
        (Utilities|Array|Add (LocalVariables|GetInputPosX) (Math|Conversions|ToInteger(Byte) (Utilities|String|GetSubstring _array_element_3 0 2)))
        (Utilities|Array|Add (LocalVariables|GetInputPosY) (Math|Conversions|ToInteger(Byte) (Utilities|String|GetSubstring _array_element_3 2 2)))
        (Utilities|Array|Add (LocalVariables|GetInputMaxHealth) 0)
        (Utilities|Array|Add (LocalVariables|GetInputAttack) 0)
        (Utilities|Array|Add (LocalVariables|GetInputCurrentHealth) 0))
      ;[1 1 1] Setup traps
      (Utilities|Array|Clear (LocalVariables|GetInputTrapID))
      (Utilities|Array|Clear (LocalVariables|GetInputTrapOwner))
      (Utilities|Array|Clear (LocalVariables|GetInputTrapLife))
      (Utilities|Array|Clear (LocalVariables|GetInputTrapPosX))
      (Utilities|Array|Clear (LocalVariables|GetInputTrapPosY))
      (for _array_element_4 (Variables|/Game/Blueprints/BP_Grid.BP_Grid_C|GetTraps (Variables|Default|GetGrid))
        (Utilities|Array|Add (LocalVariables|GetInputTrapID) (Variables|/Game/Blueprints/BP_Trap.BP_Trap_C|GetID _array_element_4))
        (Utilities|Array|Add (LocalVariables|GetInputTrapOwner) (Variables|/Game/Blueprints/BP_Entity.BP_Entity_C|GetID (Variables|/Game/Blueprints/BP_Trap.BP_Trap_C|GetScourge _array_element_4)))
        (Utilities|Array|Add (LocalVariables|GetInputTrapLife) (Variables|/Game/Blueprints/BP_Trap.BP_Trap_C|GetLife _array_element_4))
        (Utilities|Array|Add (LocalVariables|GetInputTrapPosX) (Math|Conversions|ToInteger(Byte) (Utilities|String|GetSubstring (Variables|/Game/Blueprints/BP_Trap.BP_Trap_C|GetPosition _array_element_4) 0 2)))
        (Utilities|Array|Add (LocalVariables|GetInputTrapPosY) (Math|Conversions|ToInteger(Byte) (Utilities|String|GetSubstring (Variables|/Game/Blueprints/BP_Trap.BP_Trap_C|GetPosition _array_element_4) 2 2))))
      (return (LocalVariables|GetInputNPC) (LocalVariables|GetInputNPCTeams) (LocalVariables|GetInputPosX) (LocalVariables|GetInputPosY) (LocalVariables|GetInputMaxHealth) (LocalVariables|GetInputAttack) (LocalVariables|GetInputCurrentHealth) (LocalVariables|GetInputTrapID) (LocalVariables|GetInputTrapLife) (LocalVariables|GetInputTrapOwner) (LocalVariables|GetInputTrapPosX) (LocalVariables|GetInputTrapPosY)))))