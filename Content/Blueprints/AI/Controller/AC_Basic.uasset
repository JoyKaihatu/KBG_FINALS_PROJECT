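; AC_Basic is an AI controller for BP_Entity pawns in a turn-based system.
; On possess it stores the entity, runs BT_Base and sets the blackboard Turn flag to false.
; ChangeTurn writes whether the entity can move into that flag and clears the pawn's TargetUnit.
; GetBestAction is an empty stub with disconnected initialization nodes for depth and action value.
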(event Custom|ChangeTurn
  (params (CanMove? :type Boolean))
  (AI|Components|Blackboard|SetValueasBool (AI|GetBlackboard 0) (Utilities|Name|MakeLiteralName "Turn") CanMove?)
  (Utilities|Array|Clear (Variables|/Game/Blueprints/BP_Entity.BP_Entity_C|GetTargetUnit (Variables|Default|GetControlledPawn))))

(event EventPossess
  (params (PossessedPawn :type Pawn%20Object%20Reference))
  (bind _asbp_entity (Utilities|Casting|CastToBP_Entity PossessedPawn))
  (Variables|Default|SetControlledPawn _asbp_entity)
  (AI|RunBehaviorTree "/Game/Blueprints/AI/BehaviorTree/BT_Base.BT_Base")
  (AI|Components|Blackboard|SetValueasBool (AI|GetBlackboard 0) (Utilities|Name|MakeLiteralName "Turn") false))

(fn ConstructionScript)

(fn GetBestAction)