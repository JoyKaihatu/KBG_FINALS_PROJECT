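; BP_Lich is the Lich Blueprint, which randomizes its own combat stats when play begins.
; After calling the parent BeginPlay, it rolls MaxHealth and Attack within fixed integer ranges and sets Health to full.
; It adds no other logic: overlap and Tick are disabled stubs, and the construction script only calls its parent.
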(event EventBeginPlay
  (|CallParentFunction)
  (bind _output_get (Variables|Default|SetMaxHealth (Math|Random|RandomIntegerinRange 70 90)))
  (Variables|Default|SetHealth _output_get)
  (Variables|Default|SetAttack (Math|Random|RandomIntegerinRange 20 30)))

(event Collision|EventActorBeginOverlap
  (params (OtherActor :type Actor%20Object%20Reference))
  (|CallParentFunction OtherActor) ; This node is disabled and will not be called.\nDrag off pins to build functionality.
)

(event EventTick
  (params (DeltaSeconds :type Float%20%28single-precision%29))
  (|CallParentFunction DeltaSeconds) ; This node is disabled and will not be called.\nDrag off pins to build functionality.
)

(fn ConstructionScript
  (|CallParentFunction))