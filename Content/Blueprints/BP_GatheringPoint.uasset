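; BP_GatheringPoint marks a gathering location in the level and supplies positions around it.
; On BeginPlay, a point flagged IsStartingPoint registers itself as the CurrentGatheringPoint on PC_PlayerController.
; GetValidPosition returns a random navigable location around the actor, using the ViableLocations sphere radius as the search range.
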(event EventBeginPlay
  (if (Variables|Default|GetIsStartingPoint)
    (bind _aspc_player_controller (Utilities|Casting|CastToPC_PlayerController (Game|GetPlayerController 0)))
    (Variables|/Game/Blueprints/PC_PlayerController.PC_PlayerController_C|SetCurrentGatheringPoint _aspc_player_controller self)))

(fn ConstructionScript)

(fn GetValidPosition
  (bind _randomlocation (Class|NavigationSystemV1|GetRandomLocationinNavigableRadius (Transformation|GetActorLocation) (Variables|/Script/Engine.SphereComponent|GetSphereRadius (Variables|Default|GetViableLocations)) 0 0))
  (return _randomlocation))