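; BP_Ally is an allied unit that flags itself as an ally on BeginPlay and selects the "Ally State Machine" for animation.
; AnyDamage prints a debug message, spawns a particle system at the actor, subtracts clamped damage from Health and updates the health indicator.
; It then jumps to the "Damaged" animation, or at zero health plays "Dead" and destroys the actor after a short delay.
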(event EventBeginPlay
  (|CallParentFunction)
  (bind _output_get (Variables|Default|SetAlly? true))
  (Development|PrintString (Utilities|String|ToString(Boolean) _output_get))
  (Variables|Default|SetAnimStateMachine "Ally State Machine"))

(event Collision|EventActorBeginOverlap
  (params (OtherActor :type Actor%20Object%20Reference))
  (|CallParentFunction OtherActor) ; This node is disabled and will not be called.\nDrag off pins to build functionality.
)

(event EventTick
  (params (DeltaSeconds :type Float%20%28single-precision%29))
  (|CallParentFunction DeltaSeconds))

(event Game|Damage|EventAnyDamage
  (params (Damage :type Float%20%28single-precision%29) (DamageType :type Damage%20Type%20Object%20Reference) (InstigatedBy :type Controller%20Object%20Reference) (DamageCauser :type Actor%20Object%20Reference))
  ;[0 1 0.7561] Simple damage calculation
  (Development|PrintString (Utilities|String|Append (Utilities|GetDisplayName self) ": got hit"))
  (Niagara|SpawnSystematLocation 0 (Transformation|GetActorLocation))
  (bind _output_get (Variables|Default|SetHealth (Math|Integer|Clamp(Integer) (Math|Float|Truncate (- (Variables|Default|GetHealth) Damage)) 0 (Variables|Default|GetHealth))))
  (Default|UpdateHealth (Variables|Default|GetRef_HealthIndicator) _output_get (Variables|Default|GetMaxHealth))
  (if (<= (Variables|Default|GetHealth) 0)
    (CallFunction|JumptoAnim "Dead")
    (Utilities|FlowControl|Delay 1.0)
    (Actor|DestroyActor)
    (else
      (CallFunction|JumptoAnim "Damaged"))))

(fn ConstructionScript
  (|CallParentFunction))