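; Turn-based combat grid that owns the slots, tracks units on them and rolls weighted clear rewards.
; The construction script spawns BP_GridSlot child actors into a map keyed by XXYY position strings, which range checks parse to find and highlight slots.
; Setup links TurnManager, controller and slots, placing the party randomly near a fixed start cell.
; Units can be spawned or removed by position, and RemoveUnit ends combat on a win or loss.
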(event Custom|RemoveUnit
  (params (Item :type BP%20Entity%20Object%20Reference%20%28by%20ref%29))
  (Utilities|Array|RemoveItem (Variables|Default|GetUnitsOnGrid) Item)
  (Utilities|IsValid (Variables|Default|GetTurnManager)
    (:Is%20Valid
      (Default|RemoveUnit (Variables|Default|GetTurnManager) Item)
      (bind _winorlose (CallFunction|CheckWinCondition))
      (switch Utilities|FlowControl|Switch|SwitchonE_GameCondition _winorlose
        (:NewEnumerator0
          _)
        (:NewEnumerator1
          _))
      (Default|CombatFinished (Variables|Default|GetTurnManager)))))

(event Custom|MoveUnit
  (params (X :type Float%20%28double-precision%29) (Y :type Float%20%28double-precision%29))
  ;[1 0.204 0.7728] Old Actions
)

(event Custom|AttackUnit
  ;[1 0.204 0.7728] Old Actions
)

(event Custom|Clear%20Action
  ;[1 0.204 0.7728] Old Actions
)

(event Custom|MoveSelectedSlot
  (params (Position :type String))
  (bind _gridslots (Variables|Default|GetGridSlots))
  (bind (_value _returnvalue) (Utilities|Map|Find _gridslots Position))
  ;[1 1 1] Change selected slot
  (Sprite|SetSpriteColor (Variables|Default|GetSelectedSlot) "(R=1.000000,G=1.000000,B=1.000000,A=1.000000)")
  (if _returnvalue
    (bind _output_get (Variables|Default|SetSelectedGridSlot _value))
    (Transformation|SetRelativeLocation (Variables|Default|GetSelectedSlot) (Math|Vector|MakeVector (.X (Class|KismetMathLibrary|BreakVector3f (.location (Transformation|GetRelativeTransform _output_get)))) (.Y (Class|KismetMathLibrary|BreakVector3f (.location (Transformation|GetRelativeTransform _output_get)))) (.Z (Class|KismetMathLibrary|BreakVector3f (Variables|/Script/Engine.SceneComponent|GetRelativeLocation (Variables|Default|GetSelectedSlot))))) false true)))

(event Custom|Add%20Entity
  (params (Enemy? :type Boolean))
  (bind _self self)
  (bind _selectedgridslot (Variables|Default|GetSelectedGridSlot))
  (bind _unittospawn (Variables|Default|GetUnitToSpawn))
  (bind _returnvalue (Transformation|GetWorldLocation _selectedgridslot))
  (bind _returnvalue_2 (+ _returnvalue "0.000000,0.000000,50.000000"))
  ;[0.2709 0.1983 1] Spawn entity on the grid
  (Utilities|IsValid _selectedgridslot
    (:Is%20Valid
      (bind _asbp_grid_slot (Utilities|Casting|CastToBP_GridSlot (Variables|/Script/Engine.ChildActorComponent|GetChildActor _selectedgridslot)))
      (bind _foundactor (Default|CheckUnitonGrid _asbp_grid_slot))
      (Utilities|IsValid _foundactor
        (:Is%20Not%20Valid
          (if Enemy?
            (bind _returnvalue_3 (Game|SpawnActorfromClass _unittospawn (Math|Transform|MakeTransform _returnvalue_2 (Math|Rotator|MakeRotator 0.0 0.0 (Math|Random|RandomFloatinRange -1.8e+02 1.8e+02)) "1.000000,1.000000,1.000000") "Undefined" "MultiplyWithRoot" 0 0 5 _self (Variables|/Game/Blueprints/BP_GridSlot.BP_GridSlot_C|GetPosition _asbp_grid_slot) false 0))
            (Utilities|Array|AddUnique (Variables|Default|GetUnitsOnGrid) _returnvalue_3)
            (else
              (bind _returnvalue_4 (Game|SpawnActorfromClass _unittospawn (Math|Transform|MakeTransform _returnvalue_2 "0, 0, 0" "1.000000,1.000000,1.000000") "Undefined" "MultiplyWithRoot" 0 0 5 _self (Variables|/Game/Blueprints/BP_GridSlot.BP_GridSlot_C|GetPosition _asbp_grid_slot) false 0))
              (Utilities|Array|AddUnique (Variables|Default|GetUnitsOnGrid) _returnvalue_4))))))))

(event Custom|Setup
  (params (TurnManager :type BP%20Turn%20System%20Object%20Reference))
  (bind _gridslots (Variables|Default|GetGridSlots))
  ;[1 1 1] Setup
  (Variables|Default|SetTurnManager TurnManager)
  (Utilities|IsValid (Variables|Default|GetTurnManager)
    (:Is%20Valid
      (Default|SetUp (Variables|Default|GetTurnManager) self)
      (Sprite|SetSpriteColor (Variables|Default|GetSelectedSlot) "(R=0.000000,G=0.000000,B=0.000000,A=0.000000)")
      (bind _aspc_player_controller (Utilities|Casting|CastToPC_PlayerController (Game|GetPlayerController 0)))
      (bind _output_get (Variables|Default|SetController _aspc_player_controller))
      (Default|UpdateGridRef _output_get self)
      (CallFunction|SetupMainPartyonGrid)
      (bind _keys (Utilities|Map|Keys _gridslots))
      (for _array_element _keys
        (bind _asbp_grid_slot (Utilities|Casting|CastToBP_GridSlot (Variables|/Script/Engine.ChildActorComponent|GetChildActor (.Value (Utilities|Map|Find _gridslots _array_element)))))
        (Default|Setup _asbp_grid_slot self _array_element (Variables|Default|GetController) (Variables|Default|GetTurnManager))))))

(event EventBeginPlay
  (bind _gridslots (Variables|Default|GetGridSlots))
  (bind _turnmanager (Variables|Default|GetTurnManager))
  ;[1 1 1] Setup
  (Utilities|IsValid _turnmanager
    (:Is%20Valid
      (Default|SetUp _turnmanager self)
      (Sprite|SetSpriteColor (Variables|Default|GetSelectedSlot) "(R=0.000000,G=0.000000,B=0.000000,A=0.000000)")
      (bind _aspc_player_controller (Utilities|Casting|CastToPC_PlayerController (Game|GetPlayerController 0)))
      (bind _output_get (Variables|Default|SetController _aspc_player_controller))
      (Default|UpdateGridRef _output_get self)
      (CallFunction|SetupMainPartyonGrid)
      (bind _keys (Utilities|Map|Keys _gridslots))
      (for _array_element _keys
        (bind _asbp_grid_slot (Utilities|Casting|CastToBP_GridSlot (Variables|/Script/Engine.ChildActorComponent|GetChildActor (.Value (Utilities|Map|Find _gridslots _array_element)))))
        (Default|Setup _asbp_grid_slot self _array_element (Variables|Default|GetController) (Variables|Default|GetTurnManager))))))

(fn ConstructionScript
  (for _index (range 0 (- (Utilities|Array|Get(acopy) (Variables|Default|GetSize) 1) 1)) ; atas bawah (Y)
    (for _index_2 (range 0 (- (Utilities|Array|Get(acopy) (Variables|Default|GetSize)) 1)) ; kiri kanan (X)
      (bind _returnvalue (AddComponent|AddChildActorComponent false (Math|Transform|MakeTransform (Math|Vector|MakeVector (Math|Conversions|ToFloat(Integer) (* _index 120)) (Math|Conversions|ToFloat(Integer) (* _index_2 120)) -45.0) "0, 0, 0" "1.000000,1.000000,1.000000")))
      (ChildActorComponent|SetChildActorClass _returnvalue "/Game/Blueprints/BP_GridSlot.BP_GridSlot_C")
      (Utilities|Map|Add (Variables|Default|GetGridSlots) (Utilities|String|Append (Utilities|String|ToString(Text) (Utilities|Text|ToText(Integer) _index_2 false true 2)) (Utilities|String|ToString(Text) (Utilities|Text|ToText(Integer) _index false true 2))) _returnvalue)
      (bind _asbp_grid_slot (Utilities|Casting|CastToBP_GridSlot (Variables|/Script/Engine.ChildActorComponent|GetChildActor _returnvalue)))
      (Default|Setup _asbp_grid_slot self (Utilities|String|Append (Utilities|String|ToString(Text) (Utilities|Text|ToText(Integer) _index_2 false true 2)) (Utilities|String|ToString(Text) (Utilities|Text|ToText(Integer) _index false true 2)))))))

(fn CheckActionRange
  (params (Action :type S%20Action%20Structure) (Position :type String) (EnableClickable :type Boolean))
  (bind _range (Utilities|Struct|BreakS_Action Action))
  (bind _returnvalue (Utilities|String|GetSubstring Position 0 2))
  (bind _size (Variables|Default|GetSize))
  (bind _size_2 (Variables|Default|GetSize))
  (bind _returnvalue_2 (Math|Conversions|ToInteger(Byte) _returnvalue))
  (bind _returnvalue_3 (Utilities|String|GetSubstring Position 2 2))
  (bind _output (Utilities|Array|Get(acopy) _size_2))
  (bind _output_2 (Utilities|Array|Get(acopy) _range))
  (bind _output_3 (Utilities|Array|Get(acopy) _range 1))
  (bind _output_4 (Utilities|Array|Get(acopy) _size 1))
  (bind _returnvalue_4 (Math|Conversions|ToInteger(Byte) _returnvalue_3))
  ;[1 1 1] Check the grid aplicable for certain actions
  (for _index (range (Math|Integer|Clamp(Integer) (- _returnvalue_2 _output_2) 0 _output) (Math|Integer|Clamp(Integer) (+ _returnvalue_2 _output_2) 0 _output)) ; X loop
    (for _index_2 (range (Math|Integer|Clamp(Integer) (- _returnvalue_4 _output_3) 0 _output_4) (Math|Integer|Clamp(Integer) (+ _returnvalue_4 _output_3) 0 _output_4)) ; Y loop
      ;;[1 1 1] Get positions on the grid
      (if (.ReturnValue (Utilities|Map|Find (Variables|Default|GetGridSlots) (Utilities|String|Append (Utilities|String|ToString(Text) (Utilities|Text|ToText(Integer) _index false true 2)) (Utilities|String|ToString(Text) (Utilities|Text|ToText(Integer) _index_2 false true 2)))))
        (bind _asbp_grid_slot (Utilities|Casting|CastToBP_GridSlot (Variables|/Script/Engine.ChildActorComponent|GetChildActor (.Value (Utilities|Map|Find (Variables|Default|GetGridSlots) (Utilities|String|Append (Utilities|String|ToString(Text) (Utilities|Text|ToText(Integer) _index false true 2)) (Utilities|String|ToString(Text) (Utilities|Text|ToText(Integer) _index_2 false true 2))))))))
        (if (not EnableClickable)
          (Default|ChangeMaterial _asbp_grid_slot "/Game/Material/MI_GridTransparentRed.MI_GridTransparentRed")
          (Utilities|Array|Add (LocalVariables|GetResults) _asbp_grid_slot)
          (Utilities|Array|Add (LocalVariables|GetAltResults) (Utilities|String|Append (Utilities|String|ToString(Text) (Utilities|Text|ToText(Integer) _index false true 2)) (Utilities|String|ToString(Text) (Utilities|Text|ToText(Integer) _index_2 false true 2))))))))
  (return (LocalVariables|GetResults) (LocalVariables|GetAltResults)))

(fn ResetGridSlots
  (bind _gridslots (Variables|Default|GetGridSlots))
  ;[1 1 1] Reset grids to default material and prevent it from being selectable
  (bind _keys (Utilities|Map|Keys _gridslots))
  (for _array_element _keys
    (bind _asbp_grid_slot (Utilities|Casting|CastToBP_GridSlot (Variables|/Script/Engine.ChildActorComponent|GetChildActor (.Value (Utilities|Map|Find _gridslots _array_element)))))
    (Default|Disable/EnableAction _asbp_grid_slot false)))

(fn SetupMainPartyonGrid
  (bind _turnmanager (Variables|Default|GetTurnManager))
  (bind _availablegrids (CallFunction|CheckActionRange (Utilities|Struct|MakeS_Action "Move" (Utilities|Array|MakeArray 1 1) (Utilities|Array|MakeArray 2 2) "/Game/Sprites/Arrow__3_.Arrow__3_") "0003" false))
  (LocalVariables|SetAvailableGrids _availablegrids)
  (for _array_element (Variables|/Game/Blueprints/BP_TurnSystem.BP_TurnSystem_C|GetMainParty (Variables|Default|GetTurnManager))
    (Utilities|Array|Add (Variables|Default|GetUnitsOnGrid) _array_element)
    (bind _foundactor (Default|CheckUnitonGrid (.OutItem (Utilities|Array|Random (LocalVariables|GetAvailableGrids)))))
    (Utilities|IsValid _foundactor
      (:Is%20Valid
        (Development|PrintString "Slot occupied" true true "(R=1.000000,G=0.003259,B=0.000000,A=1.000000)" 5.0)
        (Utilities|Array|Add (LocalVariables|GetRemainingPartyMember) _array_element))
      (:Is%20Not%20Valid
        (bind _output_get (LocalVariables|SetSelectedGrid (.OutItem (Utilities|Array|Random (LocalVariables|GetAvailableGrids)))))
        (Default|PrepareforCombat _array_element self _output_get)
        (Default|AddUnit (Variables|Default|GetTurnManager) _array_element)
        (Utilities|Array|RemoveItem (LocalVariables|GetAvailableGrids) (LocalVariables|GetSelectedGrid)))))
  ;[0 1 0.7561] Just in case if they cannot find an empty grid
  (for _array_element_2 (LocalVariables|GetRemainingPartyMember)
    (bind _foundactor_2 (Default|CheckUnitonGrid (.OutItem (Utilities|Array|Random (LocalVariables|GetAvailableGrids)))))
    (Utilities|IsValid _foundactor_2
      (:Is%20Not%20Valid
        (bind _output_get_2 (LocalVariables|SetSelectedGrid (.OutItem (Utilities|Array|Random (LocalVariables|GetAvailableGrids)))))
        (Default|PrepareforCombat _array_element_2 self _output_get_2)
        (Default|AddUnit (Variables|Default|GetTurnManager) _array_element_2)
        (Utilities|Array|RemoveItem (LocalVariables|GetAvailableGrids) (LocalVariables|GetSelectedGrid)))))
  (for _array_element_3 (Variables|Default|GetUnitsOnGrid)
    (if (not (Variables|/Game/Blueprints/BP_Entity.BP_Entity_C|GetAlly? _array_element_3))
      (Default|AddUnit _turnmanager _array_element_3)
      (Variables|/Game/Blueprints/BP_Entity.BP_Entity_C|SetTurn%20Manager _array_element_3 _turnmanager))))

(fn CheckWinCondition
  (bind _turnmanager (Variables|Default|GetTurnManager))
  (bind _mainparty (Variables|/Game/Blueprints/BP_TurnSystem.BP_TurnSystem_C|GetMainParty _turnmanager))
  ;[0 1 0.7561] Check if all party members deadge
  (LocalVariables|SetAmountOfPartyRemaining (Utilities|Array|Length _mainparty))
  (for _array_element _mainparty
    (if (not (Utilities|Array|ContainsItem (Variables|Default|GetUnitsOnGrid) _array_element))
      (Math|Integer|DecrementInt (LocalVariables|GetAmountOfPartyRemaining))))
  (if (<= (LocalVariables|GetAmountOfPartyRemaining) 0)
    (return "NewEnumerator1")
    (else
      ;[1 0.003259 0] Check if there's enemies remaining
      (for _array_element_2 (Variables|Default|GetUnitsOnGrid)
        (if (not (Variables|/Game/Blueprints/BP_Entity.BP_Entity_C|GetAlly? _array_element_2))
          (return "NewEnumerator2")))
      (return "NewEnumerator0"))))

(fn GetClearRewards
  (Utilities|Array|Clear (LocalVariables|GetRewardPool))
  (for _index (range 1 (Variables|Default|GetRewardAmount))
    (LocalVariables|SetRandomChance (Math|Random|RandomFloatinRange 1.0 1e+02))
    (LocalVariables|SetBuildUpChance 0.0)
    (bind _keys (Utilities|Map|Keys (Variables|Default|GetRewardForClear)))
    (bind _array_element (Utilities|Array|ForEachLoopwithBreak _keys :!label _label)
      (:LoopBody
        (bind _output_get (LocalVariables|SetBuildUpChance (+ (LocalVariables|GetBuildUpChance) (.Value (Utilities|Map|Find (Variables|Default|GetRewardForClear) _array_element)))))
        (if (> _output_get (LocalVariables|GetRandomChance))
          (Utilities|Array|Add (LocalVariables|GetRewardPool) _array_element)
          (goto _label Break)))))
  (return (LocalVariables|GetRewardPool)))

(fn AddUnitonPos
  (Variables|Default|SetSelectedGridSlot (.Value (Utilities|Map|Find (Variables|Default|GetGridSlots) (Variables|Default|GetSpecificPos))))
  (CallFunction|AddEntity true))

(fn RemoveUnitonPos
  (bind _output_get (Variables|Default|SetSelectedGridSlot (.Value (Utilities|Map|Find (Variables|Default|GetGridSlots) (Variables|Default|GetSpecificPos)))))
  (bind _asbp_grid_slot (Utilities|Casting|CastToBP_GridSlot (Variables|/Script/Engine.ChildActorComponent|GetChildActor _output_get)))
  (bind _foundactor (Default|CheckUnitonGrid _asbp_grid_slot))
  (Actor|DestroyActor _foundactor)
  (bind _asbp_entity (Utilities|Casting|CastToBP_Entity _foundactor))
  (Utilities|Array|RemoveItem (Variables|Default|GetUnitsOnGrid) _asbp_entity))