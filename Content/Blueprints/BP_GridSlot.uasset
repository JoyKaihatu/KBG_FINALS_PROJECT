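; Clickable slot actor for a grid-based unit combat system, tracking its position and whether an obstacle blocks it.
; Line traces at construction and BeginPlay detect obstacles, tint the slot red and register it with the Grid.
; Hovering moves the Grid's selected slot, and non-left clicks add an entity.
; Move and attack helpers exist, but their click logic is disconnected, and DamageUnits compares RequestingUnit to itself, so never deals damage.
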(event Custom|ChangeMaterial
  (params (Material :type Material%20Interface%20Object%20Reference))
  ;[1 1 1] Change material to indicate cilckable
  (Rendering|Material|SetMaterial (Variables|Default|GetCube) 0 Material)
  (Utilities|FlowControl|Delay 2.0)
  (if (Variables|Default|GetBlockedByObstacle)
    (Rendering|Material|SetMaterial (Variables|Default|GetCube) 0 "/Game/Material/MI_GridTransparentRed.MI_GridTransparentRed")
    (else
      (Rendering|Material|SetMaterial (Variables|Default|GetCube) 0 "/Game/Material/MI_GridTransparentGreen.MI_GridTransparentGreen"))))

(event Custom|Disable/EnableAction
  (params (Enable? :type Boolean))
  ;[1 1 1] Enable clickable
  (Variables|Default|SetInRangeForAction Enable?))

(event Custom|OnActorBeginOverlap_Event
  (params (OverlappedActor :type Actor%20Object%20Reference) (OtherActor :type Actor%20Object%20Reference)))

(event EventBeginPlay
  (CallFunction|CheckDoesTileHasObstacle)
  (if (Variables|Default|GetBlockedByObstacle)
    (Utilities|Array|Add (Variables|/Game/Blueprints/BP_Grid.BP_Grid_C|GetGridsWithObstacles (Variables|Default|GetGrid)) (Variables|Default|GetPosition))))

(event MouseInput|EventActorBeginCursorOver
  ;[1 1 1] Indicate which slot that is being hovered
  (Default|MoveSelectedSlot (Variables|Default|GetGrid) (Variables|Default|GetPosition)))

(event MouseInput|EventActorOnClicked
  (params (ButtonPressed :type Key%20Structure))
  (if (not (== ButtonPressed "LeftMouseButton"))
    ;[1 1 1] Spawn units
    (Default|AddEntity (Variables|Default|GetGrid) false)))

(fn ConstructionScript
  (bind _cube (Variables|Default|GetCube))
  (bind _returnvalue (Transformation|GetWorldLocation _cube))
  (bind _returnvalue_2 (+ (.z _returnvalue) 9e+01))
  (bind _array_element (Utilities|Array|ForEachLoopwithBreak (LocalVariables|GetlineTracePOS) :!label _label) ; x
    (:LoopBody
      (for _array_element_2 (LocalVariables|GetlineTracePOS) ; y
        (bind _returnvalue_3 (Collision|LineTraceByChannel (Math|Vector|MakeVector (+ _array_element (.x _returnvalue)) (+ _array_element_2 (.y _returnvalue)) _returnvalue_2) (Math|Vector|MakeVector (+ _array_element (.x _returnvalue)) (+ _array_element_2 (.y _returnvalue)) (+ _returnvalue_2 25.0)) "TraceTypeQuery1" false 0 "None"))
        (if _returnvalue_3
          (Rendering|Material|SetMaterial (Variables|Default|GetCube) 0 "/Game/Material/MI_GridTransparentRed.MI_GridTransparentRed")
          (Variables|Default|SetBlockedByObstacle true)
          (goto _label Break))))
    (:Completed
      (bind _returnvalue_4 (Collision|LineTraceByChannel (Math|Vector|MakeVector (.x _returnvalue) (.y _returnvalue) (.z _returnvalue)) (Math|Vector|MakeVector (.x _returnvalue) (.y _returnvalue) (+ _returnvalue_2 3e+03)) "TraceTypeQuery3" false 0 "None"))
      (if _returnvalue_4
        (Rendering|Material|SetMaterial (Variables|Default|GetCube) 0 "/Game/Material/MI_GridTransparentRed.MI_GridTransparentRed")
        (Variables|Default|SetBlockedByObstacle true)))))

(fn Setup
  (params (Grid :type BP%20Grid%20Object%20Reference) (Position :type String) (Controller :type PC%20Player%20Controller%20Object%20Reference) (TurnManager :type BP%20Turn%20System%20Object%20Reference))
  (Variables|Default|SetGrid Grid)
  (Variables|Default|SetPosition Position)
  (Variables|Default|SetController Controller)
  (Variables|Default|SetTurnManager TurnManager))

(fn DamageUnits
  (params (RequestingUnit :type BP%20Entity%20Object%20Reference))
  (for _array_element (Variables|/Game/Blueprints/BP_Grid.BP_Grid_C|GetUnitsOnGrid (Variables|Default|GetGrid))
    (if (Utilities|Enum|Equal(Enum) (Variables|/Game/Blueprints/BP_Entity.BP_Entity_C|GetPosition _array_element) (Variables|Default|GetPosition))
      (if (!= RequestingUnit RequestingUnit)
        (Game|Damage|ApplyDamage RequestingUnit (Math|Conversions|ToFloat(Integer) (Variables|/Game/Blueprints/BP_Entity.BP_Entity_C|GetAttack RequestingUnit)) 0 0)
        (return)))))

(fn MoveUnit
  (params (RequestingUnit :type BP%20Entity%20Object%20Reference))
  (bind _targetpathfinding (Variables|Default|GetTargetPathfinding))
  (bind _returnvalue (Transformation|GetWorldLocation _targetpathfinding))
  (for _array_element (Variables|/Game/Blueprints/BP_Grid.BP_Grid_C|GetUnitsOnGrid (Variables|Default|GetGrid))
    (if (Utilities|Enum|Equal(Enum) (Variables|/Game/Blueprints/BP_Entity.BP_Entity_C|GetPosition _array_element) (Variables|Default|GetPosition))
      (return)))
  (bind _outhit (Collision|LineTraceByChannel _returnvalue (- _returnvalue "0.000000,0.000000,200.000000") "TraceTypeQuery1" false 0 "None"))
  (AI|Navigation|SimpleMovetoLocation (Variables|/Game/Blueprints/BP_Entity.BP_Entity_C|GetAIController RequestingUnit) (.location _outhit))
  (Variables|/Game/Blueprints/BP_Entity.BP_Entity_C|SetPosition RequestingUnit (Variables|Default|GetPosition))
  (Default|ClearSelectUnit (Variables|Default|GetController))
  (Default|ResetGridSlots (Variables|Default|GetGrid))
  (CallFunction|ChangeMaterial "/Game/Material/MI_GridTransparentGreen.MI_GridTransparentGreen"))

(fn CheckUnitonGrid
  (if (Variables|Default|GetBlockedByObstacle)
    (return 0)
    (else
      (for _array_element (Variables|/Game/Blueprints/BP_Grid.BP_Grid_C|GetUnitsOnGrid (Variables|Default|GetGrid))
        (if (Utilities|Enum|Equal(Enum) (Variables|/Game/Blueprints/BP_Entity.BP_Entity_C|GetPosition _array_element) (Variables|Default|GetPosition))
          (return _array_element)))
      (return 0))))

(fn CheckDoesTileHasObstacle
  (bind _cube (Variables|Default|GetCube))
  (bind _returnvalue (Transformation|GetWorldLocation _cube))
  (bind _returnvalue_2 (+ (.z _returnvalue) 9e+01))
  (bind _array_element (Utilities|Array|ForEachLoopwithBreak (LocalVariables|GetlineTracePOS) :!label _label) ; x
    (:LoopBody
      (for _array_element_2 (LocalVariables|GetlineTracePOS) ; y
        (bind _returnvalue_3 (Collision|LineTraceByChannel (Math|Vector|MakeVector (+ _array_element (.x _returnvalue)) (+ _array_element_2 (.y _returnvalue)) _returnvalue_2) (Math|Vector|MakeVector (+ _array_element (.x _returnvalue)) (+ _array_element_2 (.y _returnvalue)) (+ _returnvalue_2 25.0)) "TraceTypeQuery1" false (Variables|/Game/Blueprints/BP_Grid.BP_Grid_C|GetUnitsOnGrid (Variables|Default|GetGrid)) "None"))
        (if _returnvalue_3
          (Rendering|Material|SetMaterial (Variables|Default|GetCube) 0 "/Game/Material/MI_GridTransparentRed.MI_GridTransparentRed")
          (Variables|Default|SetBlockedByObstacle true)
          (goto _label Break))))
    (:Completed
      (bind _returnvalue_4 (Collision|LineTraceByChannel (Math|Vector|MakeVector (.x _returnvalue) (.y _returnvalue) (.z _returnvalue)) (Math|Vector|MakeVector (.x _returnvalue) (.y _returnvalue) (+ _returnvalue_2 3e+03)) "TraceTypeQuery3" false (Variables|/Game/Blueprints/BP_Grid.BP_Grid_C|GetUnitsOnGrid (Variables|Default|GetGrid)) "None"))
      (if _returnvalue_4
        (Rendering|Material|SetMaterial (Variables|Default|GetCube) 0 "/Game/Material/MI_GridTransparentRed.MI_GridTransparentRed")
        (Variables|Default|SetBlockedByObstacle true)))))