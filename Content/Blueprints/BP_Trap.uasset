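; Grid trap for a turn-based game that springs on allied units and expires over time.
; On each TurnManager next-turn call, it checks its grid slot, storing any allied occupant as TargetUnit and jumping the PaperZD state machine to Trigger.
; When the slot is empty, Life drops if the TurnManager's Scourge entry is true, destroying the trap at zero.
; On destruction it removes itself from the grid's trap list.
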(event Custom|TryToTrigger
  (bind _asbp_grid_slot (Utilities|Casting|CastToBP_GridSlot (Variables|/Script/Engine.ChildActorComponent|GetChildActor (.Value (Utilities|Map|Find (Variables|/Game/Blueprints/BP_Grid.BP_Grid_C|GetGridSlots (Variables|Default|GetGrid)) (Variables|Default|GetPosition))))))
  (bind _foundactor (Default|CheckUnitonGrid _asbp_grid_slot))
  (Utilities|IsValid _foundactor
    (:Is%20Valid
      (bind _asbp_entity (Utilities|Casting|CastToBP_Entity _foundactor))
      (if (Variables|/Game/Blueprints/BP_Entity.BP_Entity_C|GetAlly? _asbp_entity)
        (Variables|Default|SetTargetUnit _foundactor)
        (Class|PaperZDAnimInstance|JumptoNode (Variables|/Script/PaperZD.PaperZDAnimationComponent|GetAnimInstance (Variables|Default|GetPaperZDAnimation)) "Trigger" "Enemy State Machine")))
    (:Is%20Not%20Valid
      (if (.Value (Utilities|Map|Find (Variables|/Game/Blueprints/BP_TurnSystem.BP_TurnSystem_C|GetUnits (Variables|Default|GetTurnManager)) (Variables|Default|GetScourge)))
        (bind _result (Math|Integer|DecrementInt (Variables|Default|GetLife))
          (:%20%20
            (if (<= _result 0)
              (Actor|DestroyActor))))))))

(event EventDestroyed
  (Utilities|Array|RemoveItem (Variables|/Game/Blueprints/BP_Grid.BP_Grid_C|GetTraps (Variables|Default|GetGrid)) self))

(event EventBeginPlay
  (Variables|Default|SetLife 2)
  (Variables|Default|SetID (Utilities|GetDisplayName self))
  (EventDispatchers|BindEventtoNextTurnCalled (Variables|Default|GetTurnManager) (delegate Custom|TryToTrigger)))

(fn ConstructionScript)