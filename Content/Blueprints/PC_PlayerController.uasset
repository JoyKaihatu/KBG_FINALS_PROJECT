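; Player controller for a grid-based, turn-based party game, creating the main menu or master HUD by level name.
; It tracks the selected unit and action, updating the action bar and asking the grid to show action range.
; It spawns party units at gathering points, moves the party after combat, and shows rewards, reachable zones or ending credits.
; Number keys set a unit class to spawn, and R damages the first grid unit.
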(event Custom|SelectUnit
  (params (Unit :type BP%20Entity%20Object%20Reference))
  (bind _output_get (Variables|Default|SetSelectedUnit Unit))
  (Default|ChangeMaterial _output_get "/AnimationSharing/AnimSharingGreen.AnimSharingGreen")
  (Default|UpdateSelectedUnit (Variables|/Game/Widgets/WB_MasterWidget.WB_MasterWidget_C|GetWB_ActionBar (Variables|Default|GetMasterWidget)) (Variables|Default|GetSelectedUnit)))

(event Custom|SelectAction
  (params (SelectedAction :type S%20Action%20Structure))
  (Default|ResetGridSlots (Variables|Default|GetRef_Grid))
  (bind _output_get (Variables|Default|SetSelectedAction SelectedAction))
  (Default|CheckActionRange (Variables|Default|GetRef_Grid) _output_get (Variables|/Game/Blueprints/BP_Entity.BP_Entity_C|GetPosition (Variables|Default|GetSelectedUnit)) false))

(event Custom|ClearSelectUnit
  (Utilities|IsValid (Variables|Default|GetSelectedUnit)
    (:Is%20Valid
      (Default|ChangeMaterial (Variables|Default|GetSelectedUnit) "/Engine/VREditor/UI/ArrowMaterial.ArrowMaterial"))
    (:Is%20Not%20Valid
      _))
  (Variables|Default|SetSelectedUnit 0)
  (Variables|Default|SetSelectedAction "")
  (Default|UpdateSelectedUnit (Variables|/Game/Widgets/WB_MasterWidget.WB_MasterWidget_C|GetWB_ActionBar (Variables|Default|GetMasterWidget))))

(event Custom|UpdateGridRef
  (params (Ref_Grid :type BP%20Grid%20Object%20Reference))
  (Variables|Default|SetRef_Grid Ref_Grid))

(event Custom|UpdateTurnManager
  (params (TurnManager :type BP%20Turn%20System%20Object%20Reference))
  (Variables|Default|SetTurnManager TurnManager))

(event Custom|AddNewUnits
  (params (Added%20Unit :type BP%20Ally%20Class%20Reference) (NewHealth :type Integer) (NewAttack :type Integer))
  (Utilities|Array|Add (Variables|Default|GetMainParty) Added%20Unit)
  (Default|AddOwnedUnits (Variables|Default|GetMasterWidget) Added%20Unit)
  (if (and (Utilities|IsValid (Variables|Default|GetCurrentGatheringPoint)) (Utilities|IsValid (Variables|Default|GetTurnManager)))
    (bind _returnvalue (Game|SpawnActorfromClass Added%20Unit (Math|Transform|MakeTransform (Default|GetValidPosition (Variables|Default|GetCurrentGatheringPoint)) "0, 0, 0" "1.000000,1.000000,1.000000") "Undefined" "MultiplyWithRoot" 0 NewHealth NewAttack 0 "0000" false 0))
    (Default|AddMainParty (Variables|Default|GetTurnManager) _returnvalue)
    (Variables|/Game/Blueprints/BP_Ally.BP_Ally_C|SetRef_HealthIndicator _returnvalue (Default|GetLastUnitStatus (Variables|Default|GetMasterWidget)))))

(event Custom|OnCombatFinished
  (Variables|Default|SetInCombat false)
  (bind _output_get (Variables|Default|SetCurrentGatheringPoint (.Value (Utilities|Map|Find (Variables|/Game/Blueprints/BP_GatheringPoint.BP_GatheringPoint_C|GetReachableGrids (Variables|Default|GetCurrentGatheringPoint)) (Variables|Default|GetRef_Grid))))) ; Find next gathering point
  (Default|MoveAllMainParty (Variables|Default|GetTurnManager) _output_get)
  (CallFunction|UpdateGridRef))

(event Custom|RewardPlayer
  (params (RewardList :type Array%20of%20BP%20Ally%20Class%20References))
  (Default|RewardSelect (Variables|/Game/Widgets/WB_MasterWidget.WB_MasterWidget_C|GetWB_MainPartySelect (Variables|Default|GetMasterWidget)) RewardList))

(event Custom|DisplayAvailableZone
  (bind _currentgatheringpoint (Variables|Default|GetCurrentGatheringPoint))
  (bind _reachablegrids (Variables|/Game/Blueprints/BP_GatheringPoint.BP_GatheringPoint_C|GetReachableGrids _currentgatheringpoint))
  (if (Utilities|Map|IsEmpty _reachablegrids)
    (bind _returnvalue (UserInterface|CreateWidget "/Game/Widgets/WB_Credits.WB_Credits_C" 0 0))
    (UserInterface|Viewport|AddtoViewport _returnvalue 0)
    (Default|PlayEnding _returnvalue)
    (else
      (bind _keys (Utilities|Map|Keys _reachablegrids))
      (Default|ShowAvailableZone (Variables|Default|GetMasterWidget) _keys))))

(event EventBeginPlay
  (bind _returnvalue (Game|GetCurrentLevelName true))
  (if (Utilities|Enum|Equal(Enum) _returnvalue "M_MainMenu")
    (bind _returnvalue_2 (UserInterface|CreateWidget "/Game/Widgets/WB_MainMenu.WB_MainMenu_C" 0 0))
    (UserInterface|Viewport|AddtoViewport _returnvalue_2 0)
    (else
      (Variables|Default|SetbShowMouseCursor true)
      (bind _returnvalue_3 (Game|ConstructObjectfromClass "/Game/Widgets/WB_MasterWidget.WB_MasterWidget_C" self))
      (bind _output_get (Variables|Default|SetMasterWidget _returnvalue_3))
      (UserInterface|Viewport|AddtoViewport _output_get 0))))

(event Input|KeyboardEvents|R
  (params (Key :type Key%20Structure :default "None"))
  (bind _ref_grid (Variables|Default|GetRef_Grid))
  (bind _unitsongrid (Variables|/Game/Blueprints/BP_Grid.BP_Grid_C|GetUnitsOnGrid _ref_grid))
  (bind _output (Utilities|Array|Get(acopy) _unitsongrid))
  (:Pressed
    (Utilities|IsValid _output
      (:Is%20Valid
        (Game|Damage|ApplyDamage _output 1.0 0 0)))))

(event Input|KeyboardEvents|1
  (params (Key :type Key%20Structure :default "None"))
  (:Pressed
    (bind _output_get (Variables|Default|SetUnitToSpawn "/Game/Blueprints/BP_Archer.BP_Archer_C"))
    (Development|PrintString (Utilities|String|Append "Selected unit: " (Utilities|GetClassDisplayName _output_get)))))

(event Input|KeyboardEvents|2
  (params (Key :type Key%20Structure :default "None"))
  (:Pressed
    (bind _output_get (Variables|Default|SetUnitToSpawn "/Game/Blueprints/BP_Knight.BP_Knight_C"))
    (Development|PrintString (Utilities|String|Append "Selected unit: " (Utilities|GetClassDisplayName _output_get)))))

(event Input|KeyboardEvents|3
  (params (Key :type Key%20Structure :default "None"))
  (:Pressed
    (bind _output_get (Variables|Default|SetUnitToSpawn "/Game/Blueprints/BP_Skeleton.BP_Skeleton_C"))
    (Development|PrintString (Utilities|String|Append "Selected unit: " (Utilities|GetClassDisplayName _output_get)))))

(event Input|KeyboardEvents|4
  (params (Key :type Key%20Structure :default "None"))
  (:Pressed
    (bind _output_get (Variables|Default|SetUnitToSpawn "/Game/Blueprints/BP_Lich.BP_Lich_C"))
    (Development|PrintString (Utilities|String|Append "Selected unit: " (Utilities|GetClassDisplayName _output_get)))))

(fn ConstructionScript)