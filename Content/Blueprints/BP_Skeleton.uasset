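; BP_Skeleton is a skeleton character Blueprint that randomizes its combat stats when play begins.
; After calling the parent BeginPlay, it rolls MaxHealth, sets Health to that value, and rolls Attack, each roll within a fixed integer range.
; It adds no other active logic: Tick and overlap events are disabled, and the construction script only calls the parent.
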(event EventBeginPlay
  (|CallParentFunction)
  (bind _output_get (Variables|Default|SetMaxHealth (Math|Random|RandomIntegerinRange 50 70)))
  (Variables|Default|SetHealth _output_get)
  (Variables|Default|SetAttack (Math|Random|RandomIntegerinRange 5 15)))

(event Collision|EventActorBeginOverlap
  (params (OtherActor :type Actor%20Object%20Reference))
  (|CallParentFunction OtherActor) ; This node is disabled and will not be called.\nDrag off pins to build functionality.
)

(event EventTick
  (params (DeltaSeconds :type Float%20%28single-precision%29))
  (|CallParentFunction DeltaSeconds) ; This node is disabled and will not be called.\nDrag off pins to build functionality.
)

(fn ConstructionScript
  (|CallParentFunction))