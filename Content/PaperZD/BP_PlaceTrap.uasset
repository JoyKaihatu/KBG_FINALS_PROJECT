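; BP_PlaceTrap is a PaperZD animation notify that places a trap for the Scourge unit.
; When received, it casts the owning actor to BP_Scourge and spawns a BP_Trap at its target tile, passing in the grid, Scourge, tile position and turn manager.
; It then registers the trap in the grid's Traps list and clears the Scourge's target tile.
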(fn OnReceiveNotify
  (params (OwningInstance :type Paper%20ZD%20Anim%20Instance%20Object%20Reference))
  (bind _asbp_scourge (Utilities|Casting|CastToBP_Scourge (Class|PaperZDAnimInstance|GetOwningActor OwningInstance)))
  (LocalVariables|SetControlledUnit _asbp_scourge)
  (bind _returnvalue (Game|SpawnActorfromClass "/Game/Blueprints/BP_Trap.BP_Trap_C" (Math|Transform|MakeTransform (Transformation|GetActorLocation (Variables|/Game/Blueprints/BP_Scourge.BP_Scourge_C|GetTargetTile _asbp_scourge)) "0, 0, 0" "1.000000,1.000000,1.000000") "Undefined" "MultiplyWithRoot" 0 (Variables|/Game/Blueprints/BP_Entity.BP_Entity_C|GetGrid (LocalVariables|GetControlledUnit)) (LocalVariables|GetControlledUnit) (Variables|/Game/Blueprints/BP_GridSlot.BP_GridSlot_C|GetPosition (Variables|/Game/Blueprints/BP_Scourge.BP_Scourge_C|GetTargetTile (LocalVariables|GetControlledUnit))) (Variables|/Game/Blueprints/BP_Entity.BP_Entity_C|GetTurn%20Manager (LocalVariables|GetControlledUnit)) 0))
  (Utilities|Array|AddUnique (Variables|/Game/Blueprints/BP_Grid.BP_Grid_C|GetTraps (Variables|/Game/Blueprints/BP_Entity.BP_Entity_C|GetGrid (LocalVariables|GetControlledUnit))) _returnvalue)
  (Variables|/Game/Blueprints/BP_Scourge.BP_Scourge_C|SetTargetTile (LocalVariables|GetControlledUnit) 0))