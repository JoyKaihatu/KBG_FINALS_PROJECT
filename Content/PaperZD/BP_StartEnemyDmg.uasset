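; BP_StartEnemyDmg is a PaperZD animation notify that deals damage at a point in an attack animation.
; It casts the animation instance's owning actor to BP_Entity and applies its Attack as damage to every unit in its TargetUnit array.
; If that cast fails, it tries BP_Trap and damages that trap's single TargetUnit using the Attack value from its Scourge.
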(fn OnReceiveNotify
  (params (OwningInstance :type Paper%20ZD%20Anim%20Instance%20Object%20Reference))
  (bind _returnvalue (Class|PaperZDAnimInstance|GetOwningActor OwningInstance))
  (bind _asbp_entity (Utilities|Casting|CastToBP_Entity _returnvalue)
    (:then
      (for _array_element (Variables|/Game/Blueprints/BP_Entity.BP_Entity_C|GetTargetUnit _asbp_entity)
        (Game|Damage|ApplyDamage _array_element (Math|Conversions|ToFloat(Integer) (Variables|/Game/Blueprints/BP_Entity.BP_Entity_C|GetAttack _asbp_entity)) 0 0)))
    (:CastFailed
      (bind _asbp_trap (Utilities|Casting|CastToBP_Trap _returnvalue))
      (Game|Damage|ApplyDamage (Variables|/Game/Blueprints/BP_Trap.BP_Trap_C|GetTargetUnit _asbp_trap) (Math|Conversions|ToFloat(Integer) (Variables|/Game/Blueprints/BP_Entity.BP_Entity_C|GetAttack (Variables|/Game/Blueprints/BP_Trap.BP_Trap_C|GetScourge _asbp_trap))) 0 0))))